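; BP_Alarm is an alarm actor that signals with a sound and two spotlights.
; StartAlarm spawns the alarm sound at the actor and lights both spotlights, while StopAlarm silences and darkens them, with IsActive tracking the state.
; ToggleOn flips IsOn, messaging every BPI_SensorToggle actor to toggle when switched on and stopping the alarm when switched off.
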(event `Start Alarm`
  (bind _spotlight_intensity (`self.Spotlight Intensity`))
  (if (not (and (`self.IsActive`) (not (`self.IsOn`))))
    (bind _returnvalue (`GameplayStatics.SpawnSoundAtLocation` "/Game/Noises/Alarm/MS_Alarm.MS_Alarm" (`self.K2_GetActorLocation`) (struct) 1.0 1.0 0.0 null null))
    (set `self.AlarmNoise` _returnvalue)
    (set `self.IsActive` true)
    (`LightComponent.SetIntensity` (`self.SpotLight`) _spotlight_intensity)
    (`LightComponent.SetIntensity` (`self.SpotLight1`) _spotlight_intensity)))

(event `Stop Alarm`
  (if (`self.IsActive`)
    (`AudioComponent.Stop` (`self.AlarmNoise`))
    (set `self.IsActive` false)
    (`LightComponent.SetIntensity` (`self.SpotLight`) 0.0)
    (`LightComponent.SetIntensity` (`self.SpotLight1`) 0.0)))

(event `Toggle On`
  (bind _output_get (set `self.IsOn` (not (`self.IsOn`))))
  (if _output_get
    (bind _outactors (`GameplayStatics.GetAllActorsWithInterface` "/Game/Blueprints/BPI_SensorToggle.BPI_SensorToggle_C"))
    (for _array_element _outactors
      (message `/Game/Blueprints/BPI_SensorToggle.Toggle Active` _array_element))
    (else
      (`self.Stop Alarm`))))

(fn `UserConstructionScript`)