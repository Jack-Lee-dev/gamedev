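; BP_Sensor is a one-shot player detector that sets off every alarm in the level.
; DetectPlayer latches on the first actor tagged Player, plays a sensor sound, calls StartAlarm on all BP_Alarm actors and ramps a point light's intensity through a timeline.
; ToggleActive only switches on: it sets Active and clears the trigger latch, though DetectPlayer never checks Active.
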(event `Detect Player`
  (params (`Actor Detected` :type "Actor Object Reference"))
  (if (and (`self.ActorHasTag` `Actor Detected` "Player") (not (`self.BeenTriggered`)))
    (set `self.BeenTriggered` true)
    (`GameplayStatics.PlaySoundAtLocation` "/Game/Noises/Alarm/MS_Sensor.MS_Sensor" (`self.K2_GetActorLocation`) (struct) 1.0 1.0 0.0 null null null null)
    (bind _outactors (`GameplayStatics.GetAllActorsOfClass` "/Game/Blueprints/Alarms/BP_Alarm.BP_Alarm_C"))
    (for _array_element _outactors
      (bind _asbp_alarm (cast `/Game/Blueprints/Alarms/BP_Alarm` _array_element))
      (`/Game/Blueprints/Alarms/BP_Alarm.Start Alarm` _asbp_alarm))
    (bind (_direction _intensity) (`Timeline|Light Intensity` :!via `PlayFromStart`)
      (:`Update`
        (`LightComponent.SetIntensity` (`self.PointLight`) (`KismetMathLibrary.Lerp` 0.0 10000000.0 _intensity))))))

(event `/Game/Blueprints/BPI_SensorToggle.Toggle Active`
  (set `self.Active` true)
  (set `self.BeenTriggered` false))

(fn `UserConstructionScript`)