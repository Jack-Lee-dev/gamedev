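; Cone-shaped alarm sensor that sweeps back and forth to detect the player and can be switched on or off.
; A timeline rotates the sphere through an arc, pausing at each end before a FlipFlop reverses it.
; Overlaps with the detection cone pass the other actor to DetectPlayer.
; Interacting toggles the Active state, actor collision, and the visibility of the spotlight and cone.
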(event `self.ReceiveBeginPlay`
  (bind (_direction _rotation) (`Timeline|Rotation` :!label _label)
    (:`Update`
      (`SceneComponent.K2_SetRelativeRotation` (`self.Sphere`) (`KismetMathLibrary.RLerp` (struct :`Yaw` -60.0) (struct :`Yaw` 60.0) _rotation) false false))
    (:`Finished`
      (`KismetSystemLibrary.Delay` 2.0)
      (`/Engine/EditorBlueprintResources/StandardMacros.FlipFlop`
        (:`A`
          (goto _label :!via `Reverse`))
        (:`B`
          (goto _label))))))

(event `self.Detection Cone.OnComponentBeginOverlap`
  (params (OverlappedComponent :type "PrimitiveComponent Object Reference") (OtherActor :type "Actor Object Reference") (OtherComp :type "PrimitiveComponent Object Reference") (OtherBodyIndex :type Integer) (bFromSweep :type Boolean) (SweepResult :type "HitResult Structure (by ref)"))
  (`self.Detect Player` OtherActor))

(event `/Game/Blueprints/BPI_Interactions.Interact`
  (bind _returnvalue (not (`self.Active`)))
  (if _returnvalue
    (`self.SetActorEnableCollision` true)
    (else
      (`self.SetActorEnableCollision` false)))
  (`SceneComponent.SetVisibility` (`self.SpotLight`) _returnvalue true)
  (`SceneComponent.SetVisibility` (`self.Detection Cone`) _returnvalue true)
  (set `self.Active` _returnvalue))

(fn `UserConstructionScript`
  (`parent.UserConstructionScript`))