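; Airlock door actor that opens automatically five seconds after BeginPlay by animating eight mesh segments.
; The Open timeline replays for three stages, advanced by a Stage counter: rotation, relative location, then scale.
; Each update blends every segment between a fixed pitch, offset or zero scale and its current transform, using quaternion slerp for rotation and vector lerps otherwise.
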(event `self.ReceiveBeginPlay`
  (`KismetSystemLibrary.Delay` 5.0)
  (`self.Open Door`))

(event `Open Door`
  (bind _stage (`self.Stage`))
  (set `self.Stage` 0)
  (bind (_direction _open_value) (`Timeline|Open` :!label _label)
    (:`Update`
      (`self.RotateGivenSegemnt` _open_value (`self.StaticMesh1`))
      (`self.RotateGivenSegemnt` _open_value (`self.StaticMesh2`))
      (`self.RotateGivenSegemnt` _open_value (`self.StaticMesh3`))
      (`self.RotateGivenSegemnt` _open_value (`self.StaticMesh4`))
      (`self.RotateGivenSegemnt` _open_value (`self.StaticMesh5`))
      (`self.RotateGivenSegemnt` _open_value (`self.StaticMesh6`))
      (`self.RotateGivenSegemnt` _open_value (`self.StaticMesh7`))
      (`self.RotateGivenSegemnt` _open_value (`self.StaticMesh8`)))
    (:`Finished`
      (if (<= _stage 1)
        (set `self.Stage` (+ _stage 1))
        (goto _label :!via `PlayFromStart`)
        (else
          (goto _label :!via `Stop`))))))

(event `RotateGivenSegemnt`
  (params (Alpha :type "Float (double-precision)") (Mesh :type "SceneComponent Object Reference"))
  (if (== (`self.Stage`) 0)
    (`SceneComponent.K2_SetRelativeRotation` Mesh (`KismetMathLibrary.Quat_Rotator` (`KismetMathLibrary.Quat_Slerp` (`KismetMathLibrary.Conv_RotatorToQuaternion` (`KismetMathLibrary.MakeRotator` 0.0 -20.0)) (`KismetMathLibrary.Conv_RotatorToQuaternion` (`SceneComponent.RelativeRotation` Mesh)) Alpha)) false false)
    (elif (== (`self.Stage`) 1)
      (`SceneComponent.K2_SetRelativeLocation` Mesh (`KismetMathLibrary.VLerp` (0.0 50.0 150.0) (`SceneComponent.RelativeLocation` Mesh) Alpha) false false)
      (else
        (`SceneComponent.SetRelativeScale3D` Mesh (`KismetMathLibrary.VLerp` (0.0 0.0 0.0) (`SceneComponent.RelativeScale3D` Mesh) Alpha))))))

(fn `UserConstructionScript`)