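; BP_Lever is an interactable lever that plays a positional sound and animates its rotation when Interact is triggered.
; The Active flag chooses whether a timeline plays forward or reverses to lerp the lever between two angles.
; When the timeline finishes, it flips Active and sends InteractMessage to ConnectedActor if that implements BPI_Interactions.
; Otherwise, it calls ToggleOn on every BP_Alarm in the level.
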(event `Switch Lever`
  (bind _connectedactor (`self.ConnectedActor`))
  (`GameplayStatics.PlaySoundAtLocation` "/Game/Noises/Alarm/camera-sound-236021.camera-sound-236021" (`self.K2_GetActorLocation`) (struct) 1.0 1.0 0.0 "/Game/Noises/Alarm/SA_Alarm.SA_Alarm" null null null)
  (if (`self.Active`)
    (bind (_direction _rotation) (`Timeline|Timeline` :!label _label)
      (:`Update`
        (`SceneComponent.K2_SetRelativeRotation` (`self.Lever`) (`KismetMathLibrary.RLerp` (struct :`Pitch` 310.0 :`Yaw` 180.0) (struct :`Pitch` 230.0 :`Yaw` 180.0) _rotation) false false))
      (:`Finished`
        (set `self.Active` (not (`self.Active`)))
        (if (`KismetSystemLibrary.DoesImplementInterface` _connectedactor "/Game/Blueprints/BPI_Interactions.BPI_Interactions_C")
          (message `/Game/Blueprints/BPI_Interactions.Interact` _connectedactor)
          (else
            (bind _outactors (`GameplayStatics.GetAllActorsOfClass` "/Game/Blueprints/Alarms/BP_Alarm.BP_Alarm_C"))
            (for _array_element _outactors
              (`/Game/Blueprints/Alarms/BP_Alarm.Toggle On` _array_element))))))
    (else
      (goto _label :!via `Reverse`))))

(event `/Game/Blueprints/BPI_Interactions.Interact`
  (`self.Switch Lever`))

(fn `UserConstructionScript`)