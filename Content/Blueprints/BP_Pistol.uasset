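; BP_Pistol is an activatable pistol item that limits fire rate and tracks ammo, with no projectile, trace or damage logic.
; BeginPlay derives the delay between shots from RPM, dividing by 60 before the conversion to double.
; ActivateItem, when the cooldown has expired and ammo remains, spends one round, draws the remaining count as debug text and restarts the cooldown.
; Tick counts that cooldown down.
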(event `self.ReceiveBeginPlay`
  (set `self.FireDelay` (/ 1.0 (`KismetMathLibrary.Conv_IntToDouble` (/ (`self.RPM`) 60)))))

(event `/Game/Blueprints/BPI_Fire.ActivateItem`
  (if (and (<= (`self.FireBuffer`) 0.0) (> (`self.CurrentAmmo`) 0))
    (set `self.CurrentAmmo` (- (`self.CurrentAmmo`) 1.0))
    (`KismetSystemLibrary.DrawDebugString` (`self.K2_GetActorLocation`) (`KismetStringLibrary.Conv_IntToString` (`self.CurrentAmmo`)) null (struct :`R` 1.0 :`G` 1.0 :`B` 1.0 :`A` 1.0) 1.0)
    (set `self.FireBuffer` (`self.FireDelay`))))

(event `self.ReceiveTick`
  (params (DeltaSeconds :type "Float (single-precision)"))
  (bind _firebuffer (`self.FireBuffer`))
  (if (>= _firebuffer 0.0)
    (set `self.FireBuffer` (- _firebuffer DeltaSeconds))))

(fn `UserConstructionScript`)