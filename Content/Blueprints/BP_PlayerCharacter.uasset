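; Third-person player character with Enhanced Input movement, sprint, crouch, stamina-gated jumping and over-the-shoulder aiming with a socketed pistol.
; Tick lerps speed and camera arm, drains or recharges stamina after a delay, and updates the HUD.
; Aiming blocks movement input and jumping, enables firing and allows shoulder-swapped framing.
; BeenFired runs a camera multi-trace, halving interface-based damage per successive hit, with debug drawing.
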(event `self.ReceiveBeginPlay`
  (bind _childactor (`self.ChildActor`))
  (bind _user_hud (`self.User Hud`))
  (`EnhancedInputSubsystemInterface.AddMappingContext` (pcsubsystem `EnhancedInputLocalPlayerSubsystem` (`GameplayStatics.GetPlayerController` 0)) "/Game/Input/IMC_PlayerInput.IMC_PlayerInput" 0 (struct))
  (`SceneComponent.K2_AttachToComponent` _childactor (`self.Mesh`) "Weapon Socket" "KeepRelative" "KeepRelative" "KeepRelative" true)
  (bind _ashud_hud (cast `/Game/UI/HUD_HUD` (`PlayerController.GetHUD` (`GameplayStatics.GetPlayerController` 0))))
  (set `self.User Hud` _ashud_hud)
  (bind _asbp_pistol (cast `/Game/Blueprints/BP_Pistol` (`ChildActorComponent.ChildActor` _childactor)))
  (`/Game/Blueprints/BP_Pistol.Set HUD` _asbp_pistol _user_hud)
  (`/Game/UI/HUD_HUD.Update Stamina` _user_hud (`self.Stamina`))
  (`/Game/UI/HUD_HUD.Update Health` _user_hud (`self.Heallth`)))

(event `EnhancedInput|/Game/Input/IA_Movement`
  (params (ActionValue :type "Vector2D Structure") (ElapsedSeconds :type "Float (double-precision)") (TriggeredSeconds :type "Float (double-precision)") (InputAction :type "InputAction Object Reference" :default "/Game/Input/IA_Movement.IA_Movement"))
  (bind (_returnvalue_roll _returnvalue_pitch _returnvalue_yaw) (`KismetMathLibrary.BreakRotator` (`self.GetControlRotation`)))
  (bind _current_speed (`self.Current Speed`))
  (:`Triggered`
    (if (not (`self.IsAimed`))
      (set `self.MovementDirs` (`KismetMathLibrary.MakeVector` ActionValue_X ActionValue_Y))
      (`self.AddMovementInput` (`KismetMathLibrary.GetRightVector` (`KismetMathLibrary.MakeRotator` _returnvalue_roll 0.0 _returnvalue_yaw)) (* ActionValue_X _current_speed))
      (`self.AddMovementInput` (`KismetMathLibrary.GetForwardVector` (`KismetMathLibrary.MakeRotator` 0.0 0.0 _returnvalue_yaw)) (* ActionValue_Y _current_speed))))
  (:`Completed`
    (set `self.MovementDirs` (0.0 0.0 0.0))))

(event `EnhancedInput|/Game/Input/IA_Look`
  (params (ActionValue :type "Vector2D Structure") (ElapsedSeconds :type "Float (double-precision)") (TriggeredSeconds :type "Float (double-precision)") (InputAction :type "InputAction Object Reference" :default "/Game/Input/IA_Look.IA_Look"))
  (bind _currentaimrate (`self.CurrentAimRate`))
  (bind _returnvalue (* (* ActionValue_Y _currentaimrate) -1.0))
  (:`Triggered`
    (if (`self.IsAimed`)
      (set `self.CurrentAimRate` (`self.AimedSensitivityRate`))
      (else
        (set `self.CurrentAimRate` 1.0)))
    (`self.AddControllerYawInput` (* ActionValue_X _currentaimrate))
    (`self.AddControllerPitchInput` _returnvalue)
    (set `self.Aim Vertical` (`KismetMathLibrary.FClamp` (+ (`self.Aim Vertical`) (* _returnvalue 2.5)) -90.0 90.0))))

(event `self.ReceiveTick`
  (params (DeltaSeconds :type "Float (single-precision)"))
  (bind _camera_arm (`self.Camera Arm`))
  (bind _current_speed (`self.Current Speed`))
  (bind _cameravisualrate (`self.CameraVisualRate`))
  (bind _speed_change_rate (`self.Speed Change Rate`))
  (bind (_socketoffset_x _socketoffset_y) (`KismetMathLibrary.BreakVector` (`SpringArmComponent.SocketOffset` _camera_arm)))
  (bind _targetarmlength (`SpringArmComponent.TargetArmLength` _camera_arm))
  (`KismetSystemLibrary.DrawDebugString` (`self.K2_GetActorLocation`) (`KismetStringLibrary.Conv_DoubleToString` (`self.Stamina`)) null (struct :`R` 1.0 :`G` 0.831865 :`A` 1.0) 0.01)
  (set `self.IsFalling` (`NavMovementComponent.IsFalling` (`self.CharacterMovement`)))
  (if (and (not (`self.IsCrouched`)) (and (> (`self.Stamina`) 0.0) (`self.Running`)))
    (set `self.Current Speed` (`KismetMathLibrary.Lerp` _current_speed (`self.Run Rate`) _speed_change_rate))
    (set `self.Stamina` (- (`self.Stamina`) (* DeltaSeconds (`self.Stamina Drain Rate`))))
    (set `self.Stamina Recharging` false)
    (set `self.Stamina Buffer` (`self.Stamina Recharge Delay`))
    (else
      (if (not (`self.IsCrouched`))
        (set `self.Current Speed` (`KismetMathLibrary.Lerp` _current_speed (`self.Walk Rate`) _speed_change_rate))
        (else
          (set `self.Current Speed` (`KismetMathLibrary.Lerp` _current_speed (`self.Crouched Rate`) _speed_change_rate))))
      (bind _output_get (set `self.Stamina Buffer` (- (`self.Stamina Buffer`) DeltaSeconds)))
      (bind _returnvalue (<= _output_get 0.0))
      (set `self.Stamina Recharging` _returnvalue)
      (if _returnvalue
        (bind _output_get_2 (set `self.Stamina` (`KismetMathLibrary.FClamp` (+ (* DeltaSeconds (`self.Stamina Recharge Rate`)) (`self.Stamina`)) 0.0 (`self.Stamina Max`)))))))
  (`/Game/UI/HUD_HUD.Update Stamina` (`self.User Hud`) _output_get_2)
  (if (`self.IsAimed`)
    (set `SpringArmComponent.TargetArmLength` (`KismetMathLibrary.Lerp` _targetarmlength (`self.OffsetCameraDistance`) _cameravisualrate) _camera_arm)
    (set `SpringArmComponent.SocketOffset` (`KismetMathLibrary.MakeVector` 0.0 (`KismetMathLibrary.Lerp` _socketoffset_y (`self.ShoulderOffsetAmount`) (`self.ShoulderMoveRate`))) _camera_arm)
    (else
      (set `SpringArmComponent.TargetArmLength` (`KismetMathLibrary.Lerp` _targetarmlength (`self.BaseCameraDistance`) _cameravisualrate) _camera_arm)
      (set `SpringArmComponent.SocketOffset` (`KismetMathLibrary.MakeVector` 0.0 (`KismetMathLibrary.Lerp` _socketoffset_y (`self.BaseShoulderAmount`) (`self.ShoulderMoveRate`))) _camera_arm))))

(event `EnhancedInput|/Game/Input/IA_Interact`
  (params (ActionValue :type Boolean) (ElapsedSeconds :type "Float (double-precision)") (TriggeredSeconds :type "Float (double-precision)") (InputAction :type "InputAction Object Reference" :default "/Game/Input/IA_Interact.IA_Interact"))
  (:`Started`
    (for _array_element (`self.GetOverlappingActors` null)
      (if (`KismetSystemLibrary.DoesImplementInterface` _array_element "/Game/Blueprints/BPI_Interactions.BPI_Interactions_C")
        (message `/Game/Blueprints/BPI_Interactions.Interact` _array_element)))))

(event `EnhancedInput|/Game/Input/IA_Crouch`
  (params (ActionValue :type Boolean) (ElapsedSeconds :type "Float (double-precision)") (TriggeredSeconds :type "Float (double-precision)") (InputAction :type "InputAction Object Reference" :default "/Game/Input/IA_Crouch.IA_Crouch"))
  (:`Triggered`
    (set `self.IsCrouched` true))
  (:`Completed`
    (set `self.IsCrouched` false)))

(event `EnhancedInput|/Game/Input/IA_Sprint`
  (params (ActionValue :type Boolean) (ElapsedSeconds :type "Float (double-precision)") (TriggeredSeconds :type "Float (double-precision)") (InputAction :type "InputAction Object Reference" :default "/Game/Input/IA_Sprint.IA_Sprint"))
  (:`Triggered`
    (set `self.Running` true))
  (:`Completed`
    (set `self.Running` false)))

(event `EnhancedInput|/Game/Input/IA_Jump`
  (params (ActionValue :type Boolean) (ElapsedSeconds :type "Float (double-precision)") (TriggeredSeconds :type "Float (double-precision)") (InputAction :type "InputAction Object Reference" :default "/Game/Input/IA_Jump.IA_Jump"))
  (:`Triggered`
    (if (and (>= (`self.Stamina`) (`self.Jump Drain`)) (not (`self.IsAimed`)))
      (`self.Jump`)
      (set `self.Stamina Recharging` false)
      (set `self.Stamina Buffer` (`self.Stamina Recharge Delay`))
      (set `self.Stamina` (- (`self.Stamina`) (`self.Jump Drain`))))))

(event `EnhancedInput|/Game/Input/IA_Fire`
  (params (ActionValue :type Boolean) (ElapsedSeconds :type "Float (double-precision)") (TriggeredSeconds :type "Float (double-precision)") (InputAction :type "InputAction Object Reference" :default "/Game/Input/IA_Fire.IA_Fire"))
  (bind _camera (`self.Camera`))
  (:`Triggered`
    (if (`self.IsAimed`)
      (message `/Game/Blueprints/BPI_Fire.ActivateItem` (`ChildActorComponent.ChildActor` (`self.ChildActor`)) self (`SceneComponent.K2_GetComponentLocation` _camera) (`SceneComponent.GetForwardVector` _camera)))))

(event `EnhancedInput|/Game/Input/IA_Aim`
  (params (ActionValue :type Boolean) (ElapsedSeconds :type "Float (double-precision)") (TriggeredSeconds :type "Float (double-precision)") (InputAction :type "InputAction Object Reference" :default "/Game/Input/IA_Aim.IA_Aim"))
  (bind _charactermovement (`self.CharacterMovement`))
  (:`Triggered`
    (set `self.IsAimed` true)
    (set `CharacterMovementComponent.bOrientRotationToMovement` false _charactermovement)
    (set `CharacterMovementComponent.bUseControllerDesiredRotation` true _charactermovement))
  (:`Completed`
    (set `self.IsAimed` false)
    (set `CharacterMovementComponent.bOrientRotationToMovement` true _charactermovement)
    (set `CharacterMovementComponent.bUseControllerDesiredRotation` false _charactermovement)))

(event `EnhancedInput|/Game/Input/IA_Reload`
  (params (ActionValue :type Boolean) (ElapsedSeconds :type "Float (double-precision)") (TriggeredSeconds :type "Float (double-precision)") (InputAction :type "InputAction Object Reference" :default "/Game/Input/IA_Reload.IA_Reload"))
  (:`Triggered`
    (message `/Game/Blueprints/BPI_Fire.Reload` (`ChildActorComponent.ChildActor` (`self.ChildActor`)))))

(event `/Game/Blueprints/BPI_Fire.BeenFired`
  (params (Damage :type "Float (double-precision) (by ref)"))
  (bind _camera (`self.Camera`))
  (bind _returnvalue (`SceneComponent.K2_GetComponentLocation` _camera))
  (bind _outhits (`KismetSystemLibrary.LineTraceMulti` :`Start` _returnvalue :`End` (+ _returnvalue (* (`SceneComponent.GetForwardVector` _camera) 1000000.0)) :`TraceChannel` "TraceTypeQuery3" :`DrawDebugType` "Persistent"))
  (for (_array_element _array_index) _outhits
    (bind (_bblockinghit _binitialoverlap _time _distance _location _impactpoint _normal _impactnormal _physmat _hitactor) (`GameplayStatics.BreakHitResult` _array_element))
    (if (`KismetSystemLibrary.DoesImplementInterface` _hitactor "/Game/Blueprints/BPI_Damagable.BPI_Damagable_C")
      (`KismetSystemLibrary.DrawDebugString` _impactpoint "Damagable" null (struct :`R` 1.0 :`G` 1.0 :`B` 1.0 :`A` 1.0) 10.0)
      (message `/Game/Blueprints/BPI_Damagable.RecieveDamage` _hitactor (/ Damage (`KismetMathLibrary.MultiplyMultiply_FloatFloat` 2.0 (`KismetMathLibrary.Conv_IntToDouble` _array_index))))
      (else
        (`KismetSystemLibrary.DrawDebugString` _impactpoint "Not Damagable" null (struct :`R` 1.0 :`G` 1.0 :`B` 1.0 :`A` 1.0) 10.0)))))

(event `EnhancedInput|/Game/Input/IA_ShoulderSwap`
  (params (ActionValue :type Boolean) (ElapsedSeconds :type "Float (double-precision)") (TriggeredSeconds :type "Float (double-precision)") (InputAction :type "InputAction Object Reference" :default "/Game/Input/IA_ShoulderSwap.IA_ShoulderSwap"))
  (:`Triggered`
    (set `self.RightShoulder` (not (`self.RightShoulder`)))
    (set `self.ShoulderOffsetAmount` (* (`self.ShoulderOffsetAmount`) -1.0))))

(fn `UserConstructionScript`)